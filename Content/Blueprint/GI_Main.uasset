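; Game instance that procedurally builds the segment-based level and keeps registries of entities and lingering volumes.
; STARTGEN runs grammar-to-WFC generation, whose per-cell callback spawns segments chosen by adjacency DataTable row and simplified region label.
; Row lookup falls back to single-letter rows, then default hallway classes; invalid region labels spawn debug planes.
; Spawned segments are stored by grid coordinate, linked to neighbors, then post-processed.
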(event `START GEN`
  (bind _returnvalue (`AlgorithmTester.TestGrammarToWFC` (delegate `CustomEvent_0`) 12 1))
  (`self.LinkSegmentNeighbors` _returnvalue)
  (bind _values (`BlueprintMapLibrary.Map_Values` (`self.SegmentLayout`)))
  (for _array_element _values
    (`/Game/Blueprint/Env/BP_EnvSegment.PostGeneration` _array_element)))

(event `self.ReceiveInit`)

(event `CustomEvent_0`
  (params (X :type Integer) (Y :type Integer) (GenOutput :type "GenOutput Structure"))
  (bind (_row _label) (`self.GenOutputRowString` GenOutput))
  (bind _intvector2d (make `/Game/Blueprint/IntVector2D` X Y))
  (bind _returnvalue (* (`KismetMathLibrary.MakeVector` (`KismetMathLibrary.Conv_IntToDouble` X) (`KismetMathLibrary.Conv_IntToDouble` Y)) (`self.Base Segment Scale`)))
  (if (`KismetArrayLibrary.Array_Contains` (`|MakeArray` "c" "B") _label)
    (bind (_found _out_row) (`self.ParseDT_Row` _row))
    (bind (_segment_class _rotation) (`self.Validate Row` _found _out_row GenOutput)
      (:`Default`
        (bind _returnvalue_2 (`|SpawnActorFromClass` _segment_class (`KismetMathLibrary.MakeTransform` _returnvalue _rotation) "Undefined" "MultiplyWithRoot" null _intvector2d GenOutput null))
        (`BlueprintMapLibrary.Map_Add` (`self.SegmentLayout`) _intvector2d _returnvalue_2)
        (if (== _segment_class "/Game/Blueprint/Env/Pipe1/BP_Segment_Pipe1_Room_base.BP_Segment_Pipe1_Room_base_C")
          (`KismetArrayLibrary.Array_Add` (`self.BaseSegments`) (cast `/Game/Blueprint/Env/Pipe1/BP_Segment_Pipe1_Room_base` _returnvalue_2 :!pure true))))
      (:`Invalid Region Label`
        (bind _returnvalue_3 (`|SpawnActorFromClass` "/Game/Blueprint/TestEnv/BP_TestPlane.BP_TestPlane_C" (`KismetMathLibrary.MakeTransform` _returnvalue (`KismetMathLibrary.MakeRotator` 0.0)) "Undefined" "MultiplyWithRoot" null null))
        (`/Game/Blueprint/TestEnv/BP_TestPlane.SetText` _returnvalue_3 (`KismetTextLibrary.Conv_NameToText` _row))
        (`KismetSystemLibrary.PrintString` (`KismetStringLibrary.Concat_StrStr` "invalid region label: " (`.Region_Label` (break `GenOutput` GenOutput))) true true (struct :`G` 0.66 :`B` 1.0 :`A` 1.0) 14.0)))))

(fn `Add Vec2D`
  (params (` ` :type "/Game/Blueprint/IntVector2D Structure") (`  ` :type "/Game/Blueprint/IntVector2D Structure"))
  (returns (`   ` :type "/Game/Blueprint/IntVector2D Structure"))
  (return (make `/Game/Blueprint/IntVector2D` (+ ` _X_3_03C7DA134B9ADC7DB0E76DB40BCDA7F0` `  _X_3_03C7DA134B9ADC7DB0E76DB40BCDA7F0`) (+ ` _Y_5_2F09043644559DEAFBD902BBA3C328D4` `  _Y_5_2F09043644559DEAFBD902BBA3C328D4`))))

(fn `Get Random Spread`
  (params (Spread :type "Float (double-precision)"))
  (returns (ReturnValue :type "Rotator Structure"))
  (bind _returnvalue (`KismetSystemLibrary.MakeLiteralDouble` Spread))
  (bind _returnvalue_2 (* _returnvalue -1.0))
  (return (`KismetMathLibrary.MakeRotator` (`KismetMathLibrary.RandomFloatInRange` _returnvalue_2 _returnvalue) (`KismetMathLibrary.RandomFloatInRange` _returnvalue_2 _returnvalue) (`KismetMathLibrary.RandomFloatInRange` _returnvalue_2 _returnvalue))))

(fn `LinkSegmentNeighbors`
  (params (Bounds :type "WFCOutput Structure"))
  (for _index (range Bounds_ExtentX_min (+ Bounds_ExtentX_max 1))
    (for _index_2 (range Bounds_ExtentY_min (+ Bounds_ExtentY_max 1))
      (bind _intvector2d (make `/Game/Blueprint/IntVector2D` _index _index_2))
      (bind (_value _returnvalue) (`BlueprintMapLibrary.Map_Find` (`self.SegmentLayout`) _intvector2d))
      (if _returnvalue
        (for _array_element (`self.DIRECTIONS`)
          (bind (_value_2 _returnvalue_2) (`BlueprintMapLibrary.Map_Find` (`self.SegmentLayout`) (`self.Add Vec2D` _array_element _intvector2d)))
          (if _returnvalue_2
            (`/Game/Blueprint/Env/BP_EnvSegment.SetNeighbor` _value _value_2 _array_element)))))))

(fn `ParseDT_Row`
  (params (RowName :type Name))
  (returns (found :type Boolean) (`Out Row` :type "/Game/Data/Lookup/Struct_AdjacencyLookup Structure"))
  (bind _returnvalue (`|GetDataTableRow` "/Game/Data/Lookup/DT_AdjacencyLookup.DT_AdjacencyLookup" RowName)
    (:`then`
      (return true _returnvalue))
    (:`RowNotFound`
      (bind _outrownames (`DataTableFunctionLibrary.GetDataTableRowNames` "/Game/Data/Lookup/DT_AdjacencyLookup.DT_AdjacencyLookup"))
      (for _array_element _outrownames
        (bind _returnvalue_2 (`KismetStringLibrary.Conv_NameToString` _array_element))
        (if (and (== (`KismetStringLibrary.Len` _returnvalue_2) 1) (`KismetStringLibrary.EqualEqual_StrStr` _returnvalue_2 (`KismetStringLibrary.GetSubstring` (`KismetStringLibrary.Conv_NameToString` RowName))))
          (bind _returnvalue_3 (`|GetDataTableRow` "/Game/Data/Lookup/DT_AdjacencyLookup.DT_AdjacencyLookup" _array_element)
            (:`then`
              (return true _returnvalue_3)))))
      (return false (make `/Game/Data/Lookup/Struct_AdjacencyLookup` null)))))

(fn `Register Entity`
  (params (` ` :type "Actor Object Reference (by ref)"))
  (`KismetArrayLibrary.Array_AddUnique` (`self.Entities`) ` `))

(fn `RegisterLingering`
  (params (` ` :type "/Game/Blueprint/Proj/Linger/BP_Lingering Object Reference (by ref)"))
  (`KismetArrayLibrary.Array_Add` (`self.Lingerings`) ` `))

(fn `Search Lingering`
  (params (Query :type "Vector Structure"))
  (returns (Lingering :type "/Game/Blueprint/Proj/Linger/BP_Lingering Object Reference") (Found :type Boolean))
  (for _array_element (`self.Lingerings`)
    (if (> (`/Game/Blueprint/Proj/Linger/BP_Lingering.Current Radius` _array_element) (`KismetMathLibrary.Vector_Distance` (`Actor.K2_GetActorLocation` _array_element) Query))
      (return _array_element true)))
  (return null false))

(fn `Unregister Entity`
  (params (`  ` :type "Actor Object Reference (by ref)"))
  (`KismetArrayLibrary.Array_RemoveItem` (`self.Entities`) `  `))

(fn `Unregister Lingering`
  (params (` ` :type "/Game/Blueprint/Proj/Linger/BP_Lingering Object Reference"))
  (`KismetArrayLibrary.Array_RemoveItem` (`self.Lingerings`) ` `))