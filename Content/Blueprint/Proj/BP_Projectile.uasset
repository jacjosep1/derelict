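; BP_Projectile is a projectile that expires after a lifetime or on overlapping anything except its instigator or another projectile.
; Impact spawns a particle system and can escalate an existing lingering actor found through the game instance, or spawn a new one.
; It damages the hit actor, applies scaled area damage to game-instance entities within an optional radius, then destroys itself.
; InitVelocity scales the movement velocity by base and modifier values.
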(event `self.ReceiveBeginPlay`
  (`KismetSystemLibrary.Delay` (`self.Lifetime`))
  (`self.K2_DestroyActor`))

(event `self.Collision.OnComponentBeginOverlap`
  (params (OverlappedComponent :type "PrimitiveComponent Object Reference") (OtherActor :type "Actor Object Reference") (OtherComp :type "PrimitiveComponent Object Reference") (OtherBodyIndex :type Integer) (bFromSweep :type Boolean) (SweepResult :type "HitResult Structure (by ref)"))
  (bind _lingering (`self.Lingering`))
  (if (not (== OtherActor (`self.Instigator`)))
    (cast `/Game/Blueprint/Proj/BP_Projectile` OtherActor
      (:`CastFailed`
        (`|ExecutionSequence`
          (:`then_0`
            ;[0.02583 0.5998 1] Impact Particle
            (`NiagaraFunctionLibrary.SpawnSystemAtLocation` (`self.Impact Particle`) SweepResult_ImpactPoint (`KismetMathLibrary.Conv_VectorToRotator` SweepResult_Normal)))
          (:`then_1`
            ;[1 0.4282 0] Lingering
            (if (`self.bDoLingering`)
              (bind (_lingering_2 _found) (`/Game/Blueprint/GI_Main.Search Lingering` (`self.GI`) SweepResult_ImpactPoint))
              (if _found
                (`/Game/Blueprint/Proj/Linger/BP_Lingering.Escalate` _lingering_2 (`self.Lingering Escalation`) SweepResult_ImpactPoint)
                (elif (`KismetSystemLibrary.IsValidClass` _lingering)
                  (`|SpawnActorFromClass` _lingering (`KismetMathLibrary.MakeTransform` SweepResult_ImpactPoint) "Undefined" "MultiplyWithRoot" self (`self.GetInstigator`))))))
          (:`then_2`
            ;[1 0.1637 0] Damage
            (message `/Game/Blueprint/INTERFACE_Entity.Apply Damage` OtherActor (`self.Base Damage`) (`self.Instigator`))
            (if (> (`self.Damage Radius`) 0.0)
              (for _array_element (`/Game/Blueprint/GI_Main.Entities` (`self.GI`))
                (if (< (`self.GetDistanceTo` _array_element self) (`self.Damage Radius`))
                  (message `/Game/Blueprint/INTERFACE_Entity.Apply Damage` _array_element (* (`self.Base Damage`) (`self.Area Damage Mult`)) (`self.Instigator`))))))
          (:`then_3`
            (`self.K2_DestroyActor`)))))))

(fn `Init Velocity`
  (params (Scale :type "Float (double-precision)"))
  (bind _projectilemovement (`self.ProjectileMovement`))
  (set `MovementComponent.Velocity` (* (`MovementComponent.Velocity` _projectilemovement) Scale (`self.Base Velocity`) (`self.Velocity Modifier`)) _projectilemovement))

(fn `UserConstructionScript`)