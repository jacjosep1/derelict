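; BP_Lingering is a lingering area-damage actor whose intensity escalates when fed and decays over time, destroying itself at zero.
; Escalate raises the level, and its integer part selects the particle system, radius and damage per tier.
; A looping timer damages GI_Main entities within the current radius.
; It registers with GI_Main on spawn and unregisters on destruction, passing a location through Escalate without ever moving.
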(event `self.ReceiveTick`
  (params (DeltaSeconds :type "Float (single-precision)"))
  ;[0 1 0.2612] Descalation
  (set `self.Escalation` (`self.Clamp Esc` (- (`self.Escalation`) (* DeltaSeconds (`self.Descalate Rate`))))))

(event `self.ReceiveBeginPlay`
  ;[1 0.9539 0] Registration
  (`|ExecutionSequence`
    (:`then_0`
      (`/Game/Blueprint/GI_Main.RegisterLingering` (cast `/Game/Blueprint/GI_Main` (`GameplayStatics.GetGameInstance`) :!pure true) self)
      ;[1 1 1] Particle Init
      (`self.Update Particles` false)
      ;[0 1 0.2612] Descalation
      (`KismetSystemLibrary.K2_SetTimerDelegate` (delegate `Descalate`) 0.2 true))
    (:`then_1`
      ;[1 0 0] Damage
      (`KismetSystemLibrary.K2_SetTimerDelegate` (delegate `CustomEvent`) (`self.Damage Delay`) true))))

(event `self.ReceiveDestroyed`
  (bind _last_particles (`self.Last Particles`))
  ;[1 0.9539 0] Registration
  (`/Game/Blueprint/GI_Main.Unregister Lingering` (cast `/Game/Blueprint/GI_Main` (`GameplayStatics.GetGameInstance`) :!pure true) self)
  ;[1 1 1] Particle Init
  (`/Engine/EditorBlueprintResources/StandardMacros.IsValid` _last_particles
    (:`Is Valid`
      (`ActorComponent.K2_DestroyComponent` _last_particles))))

(event `Descalate`
  ;[0 1 0.2612] Descalation
  (`self.Update Particles` false)
  (if (<= (`self.Escalation`) 0.0)
    (`self.K2_DestroyActor`)))

(event `CustomEvent`
  ;[1 0 0] Damage
  (if (> (`self.Current Damage`) 0.0)
    (for _array_element (`/Game/Blueprint/GI_Main.Entities` (`self.GI`))
      (if (< (`self.GetDistanceTo` _array_element self) (`self.Current Radius`))
        (message `/Game/Blueprint/INTERFACE_Entity.Apply Damage` _array_element (`self.Current Damage`) (`self.GetInstigator`))))))

(fn `Escalate`
  (params (Amount :type "Float (double-precision)") (Location :type "Vector Structure"))
  (set `self.Escalation` (`self.Clamp Esc` (+ Amount (`self.Escalation`))))
  (`self.Update Particles` false Location))

(fn `Update Particles`
  (params (bUpdateLocation :type Boolean) (`Updated Location` :type "Vector Structure"))
  (bind _last_particles (`self.Last Particles`))
  (bind _radii (`self.Radii`))
  (bind _returnvalue (`KismetMathLibrary.FTrunc` (`self.Escalation`)))
  (bind (_value _returnvalue_2) (`BlueprintMapLibrary.Map_Find` (`self.Particles`) (`KismetMathLibrary.FTrunc` (`self.Escalation`))))
  (if (!= (`KismetMathLibrary.FTrunc` (`self.Escalation`)) (`self.LastExc`))
    (`|ExecutionSequence`
      (:`then_0`
        (`/Engine/EditorBlueprintResources/StandardMacros.IsValid` _last_particles
          (:`Is Valid`
            (`ActorComponent.Deactivate` _last_particles))))
      (:`then_1`
        (if bUpdateLocation
          (`self.K2_SetActorLocation` `Updated Location`)))
      (:`then_2`
        (if _returnvalue_2
          (`|ExecutionSequence`
            (:`then_0`
              (`/Engine/EditorBlueprintResources/StandardMacros.IsValid` _value
                (:`Is Valid`
                  (bind _returnvalue_3 (`NiagaraFunctionLibrary.SpawnSystemAtLocation` _value (`SceneComponent.K2_GetComponentLocation` (`self.Sphere`))))
                  (set `self.Last Particles` _returnvalue_3))
                (:`Is Not Valid`
                  (set `self.Last Particles` null))))
            (:`then_1`
              (set `self.LastExc` _returnvalue)
              (if (and (>= _returnvalue 0) (< _returnvalue (`KismetArrayLibrary.Array_Length` _radii)))
                (set `self.Current Radius` (`|GetArrayItem` _radii _returnvalue))
                (set `self.Current Damage` (`|GetArrayItem` (`self.Damages`) _returnvalue))))))))))

(fn `UserConstructionScript`)