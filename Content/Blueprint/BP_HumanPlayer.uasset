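; First-person human player character with movement, sprinting, night vision, HUDs and an equipped child-actor tool or weapon.
; BeginPlay registers tool and entity, then moves the player to the first base segment.
; Tick eases sprint speed, drives hand animation and applies procedural weapon sway.
; Shooting and projectile spawns run immediately for the local player and relay through server-to-client events for other copies, split by an Owned/Free check.
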(event `self.ReceiveTick`
  (params (DeltaSeconds :type "Float (single-precision)"))
  (bind _movementsway_ctr (`self.MovementSway Ctr`))
  (bind _movementsway_ctr_2 (`self.MovementSway Ctr`))
  (bind _look_sway_strength (`self.Look Sway Strength`))
  (`|ExecutionSequence`
    (:`then_0`
      (bind _asabp_hands_1 (cast `/Game/Mesh/Hands/ABP_hands1` (`SkeletalMeshComponent.GetAnimInstance` (`self.Hands`))))
      (set `/Game/Mesh/Hands/ABP_hands1.bWalk` (> (`KismetMathLibrary.VSizeSquared` (`self.GetVelocity`)) 0.1) _asabp_hands_1)
      (set `/Game/Mesh/Hands/ABP_hands1.fWalktoSprint` (`KismetMathLibrary.GetRuntimeFloatCurveValue` (`self.WalkTwoSprint Interp Curve`) (`KismetMathLibrary.MapRangeClamped` (`self.Current Sprinting Mod`) 1.0 (`self.Max Sprinting Mod`) 0.0 1.0)) _asabp_hands_1))
    (:`then_1`
      (set `CharacterMovementComponent.MaxWalkSpeed` (* (`self.Current Sprinting Mod`) (`self.Default Walk Speed`)) (`self.CharacterMovement`)))
    (:`then_2`
      (bind _output_get (set `self.Current Sprinting Mod` (`KismetMathLibrary.FInterpTo` (stale _output_get) (`KismetMathLibrary.SelectFloat` (`self.Max Sprinting Mod`) 1.0 (`self.bIsSprinting`)) (`GameplayStatics.GetWorldDeltaSeconds`) (`self.Sprint Interp Speed`)))))
    (:`then_3`
      (`SceneComponent.K2_SetRelativeLocation` _movementsway_ctr_2 (`KismetMathLibrary.VInterpTo` (`SceneComponent.RelativeLocation` _movementsway_ctr_2) (* (`KismetMathLibrary.InverseTransformDirection` (`self.GetTransform`) (`KismetMathLibrary.Normal` (`self.GetVelocity`) 0.1)) (`self.Movement Sway Strength`)) (`GameplayStatics.GetWorldDeltaSeconds`) (`self.Movement Sway Interp Speed`)) false false)
      (`SceneComponent.K2_SetRelativeRotation` _movementsway_ctr (`KismetMathLibrary.RInterpTo` (`SceneComponent.RelativeRotation` _movementsway_ctr) (`KismetMathLibrary.MakeRotator` 0.0 (* (`self.GetInputAxisValue`) _look_sway_strength) (* (`self.GetInputAxisValue`) _look_sway_strength -1.0)) (`GameplayStatics.GetWorldDeltaSeconds`) (`self.Look Sway Interp Speed`)) false false))))

(event `self.ReceiveBeginPlay`
  (`|ExecutionSequence`
    (:`then_0`
      (`self.MultiplayerState`
        (:`Owned`
          (bind _returnvalue (`|CreateWidget` "/Game/Blueprint/Widget/InGame/WG_InGameHuman.WG_InGameHuman_C" (`GameplayStatics.GetPlayerController` 0) self))
          (bind _output_get (set `self.WIDGET_Human` _returnvalue))
          (`UserWidget.AddToViewport` _output_get 0)
          (bind _returnvalue_2 (`|CreateWidget` "/Game/Blueprint/Widget/InGame/WG_InGame.WG_InGame_C" (`GameplayStatics.GetPlayerController` 0)))
          (bind _output_get_2 (set `self.WIDGET_Main` _returnvalue_2))
          (`UserWidget.AddToViewport` _output_get_2 1))))
    (:`then_1`
      ;[1 1 1] TMP
      (`/Game/Blueprint/BP_MainController.Register Tool with Inventory` (`self.Get Controller`) (`self.GetTool`)))
    (:`then_2`
      (`/Game/Blueprint/GI_Main.Register Entity` (`self.GI`) self))
    (:`then_3`
      (for _array_element (`/Game/Blueprint/GI_Main.BaseSegments` (`self.GI`))
        (`self.K2_SetActorLocation` (`self.K2_GetActorLocation` _array_element))
        (break)))))

(event `self.ReceiveDestroyed`
  (`/Game/Blueprint/GI_Main.Unregister Entity` (`self.GI`) self))

(event `/Game/Blueprint/INTERFACE_Entity.Apply Damage`
  (params (Amount :type "Float (double-precision)") (Instigator :type "Actor Object Reference"))
  (`KismetSystemLibrary.PrintString` (`KismetStringLibrary.Concat_StrStr` "Damage amount to PLAYER: " (`KismetStringLibrary.Conv_DoubleToString` Amount) " FROM " (`KismetSystemLibrary.GetDisplayName` Instigator))))

(event `InputAction|Toggle Night Vision`
  (params (Key :type "Key Structure"))
  ;[0.3125 0.295 0.3013] NV
  (:`Pressed`
    (`/Game/Blueprint/Widget/InGame/WG_InGameHuman.Start NV Toggle` (`self.WIDGET_Human`))))

(event `InputAxis|LookH`
  (params (AxisValue :type "Float (single-precision)"))
  ;[0.0588 0.5655 1] Look
  (`self.AddControllerYawInput` AxisValue))

(event `InputAction|Shoot`
  (params (Key :type "Key Structure"))
  ;[1 0.1349 0.1647] Shoot Input / Networking
  (:`Pressed`
    (`self.ShootServer`)
    (`self.MultiplayerState`
      (:`Owned`
        (`self.Shoot Local`))))
  (:`Released`
    (`self.Release Server`)
    (`self.MultiplayerState`
      (:`Owned`
        (`self.Release Local`)))))

(event `InputAxis|MoveH`
  (params (AxisValue :type "Float (single-precision)"))
  ;[0.04774 1 0.0511] Movement
  (`PawnMovementComponent.AddInputVector` (`self.CharacterMovement`) (* (`self.GetActorRightVector`) AxisValue) false))

(event `InputAxis|LookY`
  (params (AxisValue :type "Float (single-precision)"))
  ;[0.0588 0.5655 1] Look
  (`self.AddControllerPitchInput` AxisValue))

(event `ShootServer`
  ;[1 0.1349 0.1647] Shoot Input / Networking
  (`self.Shoot Client`))

(event `Shoot Client`
  ;[1 0.1349 0.1647] Shoot Input / Networking
  (`self.MultiplayerState`
    (:`Free`
      (`self.Shoot Local`))))

(event `InputAxis|MoveV`
  (params (AxisValue :type "Float (single-precision)"))
  ;[0.04774 1 0.0511] Movement
  (`PawnMovementComponent.AddInputVector` (`self.CharacterMovement`) (* (`self.GetActorForwardVector`) AxisValue) false))

(event `Key|SpaceBar`
  (params (Key :type "Key Structure"))
  (:`Pressed`
    (`AlgorithmTester.SimpleGrammar`)))

(event `Release Client`
  ;[1 0.1349 0.1647] Shoot Input / Networking
  (`self.MultiplayerState`
    (:`Free`
      (`self.Release Local`))))

(event `Release Server`
  ;[1 0.1349 0.1647] Shoot Input / Networking
  (`self.Release Client`))

(event `InputAction|Sprint`
  (params (Key :type "Key Structure"))
  ;[1 0.8011 0.06383] Sprint
  (:`Pressed`
    (set `self.bPressingSprint` true)
    (bind _returnvalue (`self.Do Camera Shake` "/Game/Blueprint/Shake/SHAKE_Sprint.SHAKE_Sprint_C"))
    (bind _output_get (set `self.Last Shake` _returnvalue)))
  (:`Released`
    (set `self.bPressingSprint` false)
    (`self.Stop Camera Shake` _output_get)))

(event `InputAction|Reload`
  (params (Key :type "Key Structure"))
  (:`Pressed`
    (`|PlayMontage` (`self.Hands`) "/Game/Mesh/Hands/MONT_hands1_BarrelChange.MONT_hands1_BarrelChange")))

(event `Anim_Fire`
  ;[1 0.06134 0.04144] Anim_Fire
  (`self.MultiplayerState`
    (:`Owned`
      (bind (_direction _recoil) (`Timeline|Anim_Fire Timeline` :!via `PlayFromStart`)
        (:`Update`
          (`SceneComponent.K2_SetRelativeLocation` (`self.FireAnim Ctr`) (* _recoil -1.0 (`KismetMathLibrary.RandomUnitVectorInConeInDegrees` (1.0 0.0 0.0) 20.0) (`KismetMathLibrary.RandomFloatInRange` 1.0 2.0) 0.4) false false))))))

(event `CALLBACK_ProjSpawn`
  ;[1 0 0.009362] CALLBACK SpawnProj
  (`self.MultiplayerState`
    (:`Owned`
      (`self.ProjSpawn_Server`)
      (`self.ProjSpawn_Local`))))

(event `ProjSpawn_Server`
  ;[1 0 0.009362] CALLBACK SpawnProj
  (`self.ProjSpawn_Client`))

(event `ProjSpawn_Client`
  ;[1 0 0.009362] CALLBACK SpawnProj
  (`self.MultiplayerState`
    (:`Free`
      (`self.ProjSpawn_Local`))))

(event `ProjSpawn_Local`
  (bind (__ _bsuccess) (`self.GetWeapon`))
  ;[1 0 0.009362] CALLBACK SpawnProj
  (if _bsuccess
    (`/Game/Blueprint/Tool/BP_Weapon.SpawnProjectile` __)))

(fn `bIsSprinting`
  (returns (` ` :type Boolean))
  (return (and (> (`self.GetInputAxisValue`) 0.3) (`self.bPressingSprint`))))

(fn `Do Camera Shake`
  (params (Shake :type "LegacyCameraShake Class Reference"))
  (returns (ReturnValue :type "LegacyCameraShake Object Reference"))
  (`self.MultiplayerState`
    (:`Owned`
      (bind _returnvalue (`LegacyCameraShake.StartLegacyCameraShake` (`GameplayStatics.GetPlayerCameraManager` 0) Shake))
      (return _returnvalue))))

(fn `Get Controller`
  (returns (` ` :type "/Game/Blueprint/BP_MainController Object Reference"))
  (return (cast `/Game/Blueprint/BP_MainController` (`self.GetController`) :!pure true)))

(fn `GetCameraRotation`
  (returns (ReturnValue :type "Rotator Structure"))
  (return (`SceneComponent.K2_GetComponentRotation` (`self.Camera`))))

(fn `GetTool`
  (returns (` ` :type "/Game/Blueprint/Tool/BP_Tool Object Reference"))
  (return (cast `/Game/Blueprint/Tool/BP_Tool` (`ChildActorComponent.ChildActor` (`self.Equipted_Tool1`)) :!pure true)))

(fn `GetWeapon`
  (returns (` ` :type "/Game/Blueprint/Tool/BP_Weapon Object Reference") (bSuccess :type Boolean))
  (bind (_asbp_weapon _bsuccess) (cast `/Game/Blueprint/Tool/BP_Weapon` (`ChildActorComponent.ChildActor` (`self.Equipted_Tool1`)) :!pure true))
  (return _asbp_weapon _bsuccess))

(fn `Multiplayer State`
  (returns (bOwned :type Boolean))
  (return (== (`GameplayStatics.GetPlayerCharacter` 0) self)))

(fn `Release Local`
  (`/Game/Blueprint/Tool/BP_Tool.Release` (`self.GetTool`)))

(fn `Shoot Local`
  (`/Game/Blueprint/Tool/BP_Tool.Shoot` (`self.GetTool`)))

(fn `Stop Camera Shake`
  (params (ShakeInstance :type "CameraShakeBase Object Reference"))
  (`self.MultiplayerState`
    (:`Owned`
      (`/Engine/EditorBlueprintResources/StandardMacros.IsValid` ShakeInstance
        (:`Is Valid`
          (`PlayerCameraManager.StopCameraShake` (`GameplayStatics.GetPlayerCameraManager` 0) ShakeInstance false))))))

(fn `Team`
  (returns (Team :type "/Game/Blueprint/E_Team Enum") (Impl :type Boolean))
  (return "NewEnumerator0" true))

(fn `TestTeleport`
  (params (location :type "Vector Structure"))
  (`/Engine/EditorBlueprintResources/StandardMacros.DoOnce` false
    (:`Completed`
      (bind (_sweephitresult _returnvalue) (`self.K2_SetActorLocation` location))
      (`KismetSystemLibrary.PrintString` (`KismetStringLibrary.Concat_StrStr` (`KismetStringLibrary.Conv_BoolToString` _returnvalue) "     TEST  TP") true true (struct :`G` 0.66 :`B` 1.0 :`A` 1.0) 9999.0))))

(fn `Toggle NV`
  (bind _nv (`self.NV`))
  (bind _output_get (set `PostProcessComponent.bEnabled` (not (`PostProcessComponent.bEnabled` _nv)) _nv))
  (`LightComponent.SetIntensity` (`self.NV_Light`) (select `bool` _output_get :`true` (`self.NV Intensity`))))

(fn `UserConstructionScript`)