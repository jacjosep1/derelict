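; BP_EnvSegment is a generated environment tile that knows its grid position and neighbors and finishes itself in PostGeneration.
; It reports periodic grid membership from X+Y to GridProperty, an empty hook here.
; With edge generation on, it spawns rotated edges per direction, chosen by substring-matching neighbor labels, with NullEdge for missing or unmatched neighbors, and runs their PostGeneration.
; Flagged segments that support turrets spawn BP_Enemy_Turret at the SPAWNTurret offset.
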(event `self.ReceiveBeginPlay`)

(fn `GridProperty`
  (params (Index :type Integer) (`On Grid` :type Boolean)))

(fn `MakeTurret`
  (if (`self.bSupportsTurrets`)
    (`|SpawnActorFromClass` "/Game/Blueprint/Enemy/Turret/BP_Enemy_Turret.BP_Enemy_Turret_C" (`KismetMathLibrary.MakeTransform` (+ (`self.K2_GetActorLocation`) (`SceneComponent.RelativeLocation` (`self.SPAWN_Turret`)))) "AlwaysSpawn" "MultiplyWithRoot" self null)))

(fn `Match Label`
  (params (Label :type "String (by ref)"))
  (returns (Found :type Boolean) (Value :type "Map of /Game/Blueprint/IntVector2D Structure to /Game/Blueprint/Env/BP_EnvSegment Class Reference"))
  (bind _edgeclassesmap (`self.EdgeClassesMap`))
  (bind _keys (`BlueprintMapLibrary.Map_Keys` _edgeclassesmap))
  (for _array_element _keys
    (if (`KismetStringLibrary.Contains` _array_element Label)
      (return true (break `/Game/Blueprint/Env/Struct_EdgeLookup` (`BlueprintMapLibrary.Map_Find` _edgeclassesmap _array_element)))))
  (return false))

(fn `PostGeneration`
  (bind (_gen_output_label _gen_output_scale _gen_output_leftlabel _gen_output_rightlabel _gen_output_uplabel _gen_output_downlabel _gen_output_hasturret) (break `GenOutput` (`self.Gen Output`)))
  (bind _position (`self.Position`))
  (bind (_position_x _position_y) (break `/Game/Blueprint/IntVector2D` (`self.Position`)))
  (`|ExecutionSequence`
    (:`then_0`
      ;[0 1 0.5032] Grid Property
      (for _index (range (`KismetArrayLibrary.Array_Length` (`self.Grid Property Sizes`)))
        (`self.GridProperty` _index (== (mod (+ _position_x _position_y) (`|GetArrayItem` (`self.Grid Property Sizes`) _index)) 0))))
    (:`then_1`
      ;[0.7552 0.2944 0.1656] Edge Generation
      (if (`self.bGenerateEdges`)
        (for _array_element (`/Game/Blueprint/GI_Main.DIRECTIONS` (cast `/Game/Blueprint/GI_Main` (`GameplayStatics.GetGameInstance`) :!pure true))
          (bind (_value _returnvalue) (`BlueprintMapLibrary.Map_Find` (`self.Neighbors`) _array_element))
          (if _returnvalue
            (`/Engine/EditorBlueprintResources/StandardMacros.IsValid` _value
              (:`Is Valid`
                (bind _gen_output_label_2 (break `GenOutput` (`/Game/Blueprint/Env/BP_EnvSegment.Gen Output` _value)))
                (bind (_found _value_2) (`self.Match Label` _gen_output_label_2))
                (if _found
                  (bind _value_3 (`BlueprintMapLibrary.Map_Find` _value_2 _array_element))
                  (if (`KismetSystemLibrary.IsValidClass` _value_3)
                    (bind _value_4 (`BlueprintMapLibrary.Map_Find` (`self.EdgeRotations`) _array_element))
                    (bind _returnvalue_2 (`KismetMathLibrary.MakeTransform` (`self.K2_GetActorLocation`) (`KismetMathLibrary.MakeRotator` 0.0 0.0 _value_4)))
                    (bind _genoutput (make `GenOutput` (`KismetStringLibrary.Conv_DoubleToString` _value_4) 1))
                    (bind _returnvalue_3 (`|SpawnActorFromClass` _value_3 _returnvalue_2 "Undefined" "MultiplyWithRoot" null _position _genoutput null))
                    (`self.PostGeneration` _returnvalue_3))
                  (else
                    (bind _returnvalue_4 (`|SpawnActorFromClass` (`self.Null Edge`) _returnvalue_2 "Undefined" "MultiplyWithRoot" null _position _genoutput null :!label _label))
                    (`self.PostGeneration` _returnvalue_4))))
              (:`Is Not Valid`
                (goto _label)))
            (else
              (goto _label))))))
    (:`then_2`
      ;[0.9723 0.5947 1] Generation Flags
      (if _gen_output_hasturret
        (`self.MakeTurret`)))))

(fn `SetNeighbor`
  (params (Neighbor :type "/Game/Blueprint/Env/BP_EnvSegment Object Reference") (Dir :type "/Game/Blueprint/IntVector2D Structure"))
  (`BlueprintMapLibrary.Map_Add` (`self.Neighbors`) Dir Neighbor))

(fn `UserConstructionScript`)