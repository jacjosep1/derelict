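; Base Blueprint for a Pipe1 room segment in a generated environment, with a test hook that teleports the player to rooms containing a turret.
; After the parent's post-generation step, it starts a wait event that delays two seconds.
; If the player pawn is valid and the generation output has a turret, it calls the human player's test teleport with the segment's location.
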(event `gen_wait`
  (bind _returnvalue (`GameplayStatics.GetPlayerPawn` 0))
  (bind (_gen_output_label _gen_output_scale _gen_output_leftlabel _gen_output_rightlabel _gen_output_uplabel _gen_output_downlabel _gen_output_hasturret) (break `GenOutput` (`self.Gen Output`)))
  (`KismetSystemLibrary.Delay` 2.0)
  (`/Engine/EditorBlueprintResources/StandardMacros.IsValid` _returnvalue
    (:`Is Valid`
      (if _gen_output_hasturret
        (bind _asbp_human_player (cast `/Game/Blueprint/BP_HumanPlayer` _returnvalue))
        (`/Game/Blueprint/BP_HumanPlayer.TestTeleport` _asbp_human_player (`self.K2_GetActorLocation`))))))

(fn `PostGeneration`
  (`parent.PostGeneration`)
  (`self.gen_wait`))

(fn `UserConstructionScript`
  (`parent.UserConstructionScript`))