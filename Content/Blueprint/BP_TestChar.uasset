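; BP_TestChar is a test character Blueprint that pairs basic player controls with a trigger for procedural generation experiments.
; Axis inputs feed movement along the actor's forward and right vectors and drive controller yaw and pitch.
; Space Bar calls SimpleGrammar, which is defined outside this graph.
; A SimpleImageWFC call seeded by DT_TestSeed is left disconnected and never runs.
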(event `InputAxis|MoveH`
  (params (AxisValue :type "Float (single-precision)"))
  (`PawnMovementComponent.AddInputVector` (`self.CharacterMovement`) (* (`self.GetActorRightVector`) AxisValue) false))

(event `InputAxis|LookH`
  (params (AxisValue :type "Float (single-precision)"))
  (`self.AddControllerYawInput` AxisValue))

(event `InputAxis|LookY`
  (params (AxisValue :type "Float (single-precision)"))
  (`self.AddControllerPitchInput` AxisValue))

(event `Key|SpaceBar`
  (params (Key :type "Key Structure"))
  (:`Pressed`
    (`AlgorithmTester.SimpleGrammar`)))

(event `InputAxis|MoveV`
  (params (AxisValue :type "Float (single-precision)"))
  (`PawnMovementComponent.AddInputVector` (`self.CharacterMovement`) (* (`self.GetActorForwardVector`) AxisValue) false))

(fn `UserConstructionScript`)