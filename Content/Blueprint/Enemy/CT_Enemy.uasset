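; Enemy AI controller that runs a behavior tree on possess and picks targets through AI Perception.
; Perception updates use a team interface to filter out same-team actors and one excluded team value, then add or remove the rest from a perceived list.
; Each change re-selects the closest perceived actor by distance and writes it to the blackboard as the current target.
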(event `self.ReceivePossess`
  (params (PossessedPawn :type "Pawn Object Reference"))
  (`self.RunBehaviorTree` (`self.Behavior Tree`)))

(event `self.AIPerception.OnTargetPerceptionUpdated`
  (params (Actor :type "Actor Object Reference") (Stimulus :type "AIStimulus Structure"))
  (bind _perceived_targets (`self.Perceived Targets`))
  ;[0.2333 1 0.3191] AI Perception
  (bind (_team _impl) (message `/Game/Blueprint/INTERFACE_Entity.Team` Actor))
  (if (and (`|EnumInequality` _team "NewEnumerator3") _impl (`|EnumInequality` _team (`self.Get Team`)))
    (if (`.bSuccessfullySensed` (break `AIStimulus` Stimulus))
      (`KismetArrayLibrary.Array_AddUnique` _perceived_targets Actor)
      (`self.Update Current Target`)
      (else
        (`KismetArrayLibrary.Array_RemoveItem` _perceived_targets Actor)
        (`self.Update Current Target`)))))

(fn `Find Closest Target`
  (returns (Closest :type "Actor Object Reference"))
  (locals (`Min Dist` :type "Float (double-precision)" :default 99999999.0) (Return :type "Actor Object Reference"))
  (for _array_element (`self.Perceived Targets`)
    (bind _returnvalue (`KismetMathLibrary.Vector_Distance` (`self.K2_GetActorLocation` _array_element) (`self.K2_GetActorLocation`)))
    (if (< _returnvalue (`local.Min Dist`))
      (set `local.Min Dist` _returnvalue)
      (set `local.Return` _array_element)))
  (return (`local.Return`)))

(fn `Get Team`
  (returns (` ` :type "/Game/Blueprint/E_Team Enum"))
  (return (`self.Default Team`)))

(fn `Update Current Target`
  (bind _closest (`self.Find Closest Target`))
  (set `self.Current Target` _closest)
  (`BlackboardComponent.SetValueAsObject` (`AIBlueprintHelperLibrary.GetBlackboard` null) (`self.Target Name`) _closest))

(fn `UserConstructionScript`)