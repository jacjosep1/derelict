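; Base enemy actor Blueprint that registers itself as an entity on BeginPlay and unregisters when destroyed, through a GI helper.
; Team queries read the team from a validated CT_Enemy controller, falling back to a fixed enum value when none is valid.
; The ApplyDamage event only prints the amount and instigator, with no health or death logic.
; The GI graph's cast to GI_Main is left unconnected.
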(event `self.ReceiveBeginPlay`
  (`/Game/Blueprint/GI_Main.Register Entity` (`self.GI`) self))

(event `self.ReceiveDestroyed`
  (`/Game/Blueprint/GI_Main.Unregister Entity` (`self.GI`) self))

(event `/Game/Blueprint/INTERFACE_Entity.Apply Damage`
  (params (Amount :type "Float (double-precision)") (Instigator :type "Actor Object Reference"))
  (`KismetSystemLibrary.PrintString` (`KismetStringLibrary.Concat_StrStr` "Damage amount to ENEMY: " (`KismetStringLibrary.Conv_DoubleToString` Amount) " FROM " (`KismetSystemLibrary.GetDisplayName` Instigator))))

(fn `Get Controller`
  (returns (` ` :type "/Game/Blueprint/Enemy/CT_Enemy Object Reference") (Valid :type Boolean))
  (bind _returnvalue (`self.GetController`))
  (bind (_asct_enemy _bsuccess) (cast `/Game/Blueprint/Enemy/CT_Enemy` _returnvalue :!pure true))
  (`/Engine/EditorBlueprintResources/StandardMacros.IsValid` _returnvalue
    (:`Is Valid`
      (if _bsuccess
        (return _asct_enemy true)
        (else
          _)))
    (:`Is Not Valid`
      _))
  (return null false))

(fn `Team`
  (returns (Team :type "/Game/Blueprint/E_Team Enum") (Impl :type Boolean))
  (bind (__ _valid) (`self.Get Controller`))
  (if _valid
    (return (`/Game/Blueprint/Enemy/CT_Enemy.Get Team` __) true)
    (else
      (return "NewEnumerator3" true))))

(fn `UserConstructionScript`)