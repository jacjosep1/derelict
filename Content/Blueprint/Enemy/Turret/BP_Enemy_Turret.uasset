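; Enemy turret that aims at a given point and fires timed volleys of spread bullets with muzzle effects.
; RotateToPoint sets a target rotation that Tick applies directly to yaw and pitch bones on intact and destroyed poseable meshes.
; Volleys run locally on server and remotes, using a chargeup delay and looping shot timer; only authority fires the completion callback.
; Death swaps in the destroyed mesh with an effect and halts aiming and shooting.
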(event `self.ReceiveBeginPlay`
  (`parent.ReceiveBeginPlay`))

(event `Do Attack Volley Multi`
  ;[1 0.04943 0] Attack Volley
  (`/Engine/EditorBlueprintResources/ActorMacros.Switch Has Authority`
    (:`Remote`
      (`self.Do Attack Volley Local` null))))

(event `DoAttackVolley`
  (params (Callback :type "/Game/Blueprint/Enemy/Turret/Task/BTTask_Turret_Volley Object Reference"))
  ;[1 0.04943 0] Attack Volley
  (`self.Do Attack Volley Multi`)
  (`self.Do Attack Volley Local` Callback))

(event `Do Attack Volley Local`
  (params (Callback :type "/Game/Blueprint/Enemy/Turret/Task/BTTask_Turret_Volley Object Reference"))
  ;[1 0.04943 0] Attack Volley
  (set `self.Last Volley Callback` Callback)
  (`KismetSystemLibrary.Delay` (`self.Volley Chargeup`))
  (bind _returnvalue (`KismetSystemLibrary.K2_SetTimerDelegate` (delegate `CustomEvent`) (`self.Shot Delay`) true))
  (bind _output_get (set `self.Last Volley Timer` _returnvalue))
  (`KismetSystemLibrary.Delay` (`self.Volley Length`))
  (`KismetSystemLibrary.K2_ClearAndInvalidateTimerHandle` _output_get)
  (`/Engine/EditorBlueprintResources/ActorMacros.Switch Has Authority`
    (:`Authority`
      (`/Game/Blueprint/Enemy/Turret/Task/BTTask_Turret_Volley.CALLBACK` (`self.Last Volley Callback`)))))

(event `self.ReceiveTick`
  (params (DeltaSeconds :type "Float (single-precision)"))
  (bind _poseablemesh (`self.PoseableMesh`))
  (bind (_target_rotation_roll _target_rotation_pitch _target_rotation_yaw) (`KismetMathLibrary.BreakRotator` (`self.Target Rotation`)))
  (bind _returnvalue (+ _target_rotation_yaw 90.0))
  (`parent.ReceiveTick` DeltaSeconds)
  ;[0.9775 1 0] Rotation Interp
  (`PoseableMeshComponent.SetBoneRotationByName` _poseablemesh (`self.Yaw Rotator Bone`) (`KismetMathLibrary.MakeRotator` 0.0 -90.0 _returnvalue) "WorldSpace")
  (`PoseableMeshComponent.SetBoneRotationByName` (`self.PoseableMesh_Dest`) (`self.Yaw Rotator Bone`) (`KismetMathLibrary.MakeRotator` 0.0 -90.0 _returnvalue) "WorldSpace")
  (`PoseableMeshComponent.SetBoneRotationByName` _poseablemesh (`self.Pitch Rotator Bone`) (`KismetMathLibrary.MakeRotator` _target_rotation_pitch 0.0 _returnvalue) "WorldSpace")
  (`PoseableMeshComponent.SetBoneRotationByName` (`self.PoseableMesh_Dest`) (`self.Pitch Rotator Bone`) (`KismetMathLibrary.MakeRotator` _target_rotation_pitch 0.0 _returnvalue) "WorldSpace"))

(event `CustomEvent`
  ;[1 0.04943 0] Attack Volley
  (if (not (`self.bDead`))
    (bind _returnvalue (`|SpawnActorFromClass` "/Game/Blueprint/Proj/Projectiles/BP_Projectile_Bullet.BP_Projectile_Bullet_C" (`KismetMathLibrary.MakeTransform` (`SceneComponent.GetSocketLocation` (`self.PoseableMesh`) "FP") (`KismetMathLibrary.ComposeRotators` (`self.Target Rotation`) (`/Game/Blueprint/GI_Main.Get Random Spread` (`self.GI`) (`self.Shot Spread`)))) "AlwaysSpawn" "MultiplyWithRoot" self 1.0 0.0 10.0 50.0 0.5 self))
    (`/Engine/EditorBlueprintResources/StandardMacros.IsValid` _returnvalue
      (:`Is Valid`
        (`/Game/Blueprint/Proj/BP_Projectile.Init Velocity` _returnvalue 30.0))
      (:`Is Not Valid`
        _))
    (`NiagaraFunctionLibrary.SpawnSystemAtLocation` "/Game/FX/MF/N_MF_Turret_Bullet.N_MF_Turret_Bullet" (`SceneComponent.GetSocketLocation` (`self.PoseableMesh`) "MF") (`self.Target Rotation`))))

(fn `Perform Death`
  (`parent.Perform Death`)
  (`SceneComponent.SetVisibility` (`self.PoseableMesh`) false true)
  (`SceneComponent.SetVisibility` (`self.PoseableMesh_Dest`) true true)
  (`NiagaraFunctionLibrary.SpawnSystemAtLocation` (`self.Death Effect`) (`self.K2_GetActorLocation`)))

(fn `Rotate to Point`
  (params (Target :type "Vector Structure"))
  (if (not (`self.bDead`))
    (bind _returnvalue (`PoseableMeshComponent.GetBoneLocationByName` (`self.PoseableMesh`) (`self.Base Bone`) "WorldSpace"))
    (set `self.Target Rotation` (`KismetMathLibrary.FindLookAtRotation` _returnvalue Target))))

(fn `UserConstructionScript`
  (`parent.UserConstructionScript`))