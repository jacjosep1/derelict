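; BP_MainController keeps the active inventory of tools and cools their heat over time.
; RegisterToolWithInventory wraps a tool in a new BP_ActiveInventoryEntry, adds it to ActiveInventory and hands the entry back to the tool.
; Each Tick, it calls CoolHeat on every entry with the frame's delta time.
; BeginPlay and the construction script perform no work.
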(event `self.ReceiveBeginPlay`
  (`|ExecutionSequence`))

(event `self.ReceiveTick`
  (params (DeltaSeconds :type "Float (single-precision)"))
  (`|ExecutionSequence`
    (:`then_0`
      (for _array_element (`self.ActiveInventory`)
        (`/Game/Blueprint/Tool/BP_ActiveInventoryEntry.Cool Heat` _array_element (`GameplayStatics.GetWorldDeltaSeconds`))))))

(fn `Register Tool with Inventory`
  (params (Tool :type "/Game/Blueprint/Tool/BP_Tool Object Reference"))
  (bind _returnvalue (`|GenericCreateObject` "/Game/Blueprint/Tool/BP_ActiveInventoryEntry.BP_ActiveInventoryEntry_C" Tool))
  (`KismetArrayLibrary.Array_Add` (`self.ActiveInventory`) _returnvalue)
  (`/Game/Blueprint/Tool/BP_Tool.Register Inventory Item` Tool _returnvalue))

(fn `UserConstructionScript`)