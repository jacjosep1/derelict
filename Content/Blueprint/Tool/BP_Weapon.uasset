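; Plasma weapon Blueprint that fires automatically while shoot is held, builds heat per shot and stops firing when overheated.
; Tick runs a delay-gated firing macro that triggers the owner's animation and camera shake, a muzzle flash and AddHeat.
; Each shot either calls back to the owning player for synced spawning or directly spawns a plasma projectile along camera rotation with random spread.
; BeginPlay puts a dynamic material on the overheat bar.
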(event `self.ReceiveBeginPlay`
  (`parent.ReceiveBeginPlay`)
  (`|ExecutionSequence`
    (:`then_0`
      (bind _returnvalue (`KismetMaterialLibrary.CreateDynamicMaterialInstance` "/Game/Material/UI/MI_OverheatBar_EDI.MI_OverheatBar_EDI"))
      (bind _output_get (set `self.OverheatBar Mat` _returnvalue))
      (`PrimitiveComponent.SetMaterial` (`self.OverheatBar`) 0 _output_get))))

(event `self.ReceiveTick`
  (params (DeltaSeconds :type "Float (single-precision)"))
  (bind __ (`self.Player Owner`))
  (`parent.ReceiveTick` DeltaSeconds)
  (`|ExecutionSequence`
    (:`then_0`
      (if (and (not (`self.bFiringControl`)) (`self.bPressingShoot`) (not (`self.Heat Info`)))
        (set `self.bFiringControl` true)
        (`|ExecutionSequence`
          (:`then_0`
            (`KismetSystemLibrary.Delay` 0.07)
            (set `self.bFiringControl` false))
          (:`then_1`
            (`/Game/Blueprint/BP_HumanPlayer.Anim_Fire` __)
            (`/Game/Blueprint/BP_HumanPlayer.Do Camera Shake` __ "/Game/Blueprint/Shake/SHAKE_Small.SHAKE_Small_C")
            (`self.Muzzle Flash Event`)
            (`|ExecutionSequence`
              (:`then_0`
                (if (`self.BSyncEachShot`)
                  (`/Game/Blueprint/BP_HumanPlayer.CALLBACK_ProjSpawn` (`self.Player Owner`))
                  (else
                    (`self.SpawnProjectile`))))
              (:`then_1`
                (`self.Add Heat`)))))))))

(event `Muzzle Flash Event`
  (`NiagaraFunctionLibrary.SpawnSystemAttached` "/Game/FX/MF/N_MF_Plasma.N_MF_Plasma" (`self.Muzzle`) "MF" (0.0 0.0 0.0) (struct) "SnapToTarget" true)
  (bind (_direction _intensity_mult) (`Timeline|MF Light Timeline` :!via `PlayFromStart`)
    (:`Update`
      (`LightComponent.SetIntensity` (`self.MuzzleFlashLight`) (* _intensity_mult 3000.0)))))

(fn `SpawnProjectile`
  (bind __ (`self.Player Owner`))
  (bind _returnvalue (`|SpawnActorFromClass` "/Game/Blueprint/Proj/Projectiles/BP_Projectile_Plasma.BP_Projectile_Plasma_C" (`KismetMathLibrary.MakeTransform` (`SceneComponent.K2_GetComponentLocation` (`self.FirePoint`)) (`KismetMathLibrary.ComposeRotators` (`/Game/Blueprint/BP_HumanPlayer.GetCameraRotation` (`self.Player Owner`)) (`/Game/Blueprint/GI_Main.Get Random Spread` (`self.GI`) 0.6))) "AlwaysSpawn" "MultiplyWithRoot" __ 1.0 0.2 10.0 0.0 0.0 __))
  (`/Game/Blueprint/Proj/BP_Projectile.Init Velocity` _returnvalue 30.0))

(fn `UserConstructionScript`
  (`parent.UserConstructionScript`))