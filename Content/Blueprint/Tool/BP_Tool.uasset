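; BP_Tool is a player-held tool, apparently a base class, with chargeable firing and overheat feedback.
; Shoot sets PressingShoot immediately or after a ChargeupTime timer, and Release clears both the flag and the pending timer.
; Heat lives on the registered InventoryItem: AddHeat adds to it, and Tick copies it into the overheat bar's material parameters.
; PlayerOwner resolves the BP_HumanPlayer through the root's attach parent, and BSyncEachShot returns false.
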(event `self.ReceiveTick`
  (params (DeltaSeconds :type "Float (single-precision)"))
  (bind (_overheated _current_heat) (`self.Heat Info`))
  (`|ExecutionSequence`
    (:`then_0`
      (`self.Update Overheat Bar` _current_heat _overheated))))

(event `Shoot Event`
  (bind _chargeup_time (`self.Chargeup Time`))
  ;[0.1645 1 0.5005] Shoot Chargeup
  (if (`KismetMathLibrary.NearlyEqual_FloatFloat` _chargeup_time)
    (set `self.bPressingShoot` true :!label _label)
    (else
      (bind _returnvalue (`KismetSystemLibrary.K2_SetTimerDelegate` (delegate `Shoot Event Delay`) _chargeup_time))
      (set `self.Shoot Event Handle` _returnvalue))))

(event `Shoot Event Delay`
  ;[0.1645 1 0.5005] Shoot Chargeup
  (goto _label))

(fn `Add Heat`
  (`/Game/Blueprint/Tool/BP_ActiveInventoryEntry.Add Heat` (`self.Inventory Item`) (`self.Heat Buildup`)))

(fn `BSyncEachShot`
  (returns (` ` :type Boolean))
  (return false))

(fn `Heat Info`
  (returns (Overheated :type Boolean) (`Current Heat` :type "Float (double-precision)"))
  (bind _inventory_item (`self.Inventory Item`))
  (bind (_overheated _current_heat) (`/Game/Blueprint/Tool/BP_ActiveInventoryEntry.Heat Info` _inventory_item))
  (`/Engine/EditorBlueprintResources/StandardMacros.IsValid` _inventory_item
    (:`Is Valid`
      (return _overheated _current_heat))
    (:`Is Not Valid`
      (return false 0.0))))

(fn `Player Owner`
  (returns (` ` :type "/Game/Blueprint/BP_HumanPlayer Object Reference") (Success :type Boolean))
  (bind _asbp_human_player (cast `/Game/Blueprint/BP_HumanPlayer` (`ActorComponent.GetOwner` (`SceneComponent.GetAttachParent` (`self.DefaultSceneRoot`))))
    (:`then`
      (return _asbp_human_player true))
    (:`CastFailed`
      (return null false))))

(fn `Register Inventory Item`
  (params (`Inventory Item` :type "/Game/Blueprint/Tool/BP_ActiveInventoryEntry Object Reference"))
  (set `self.Inventory Item` `Inventory Item`))

(fn `Release`
  (set `self.bPressingShoot` false)
  (if (`KismetSystemLibrary.K2_IsValidTimerHandle` (`self.Shoot Event Handle`))
    (`KismetSystemLibrary.K2_ClearAndInvalidateTimerHandle` (`self.Shoot Event Handle`))))

(fn `Shoot`
  (`self.Shoot Event`))

(fn `Update Overheat Bar`
  (params (Progress :type "Float (double-precision)") (Overheated :type Boolean))
  (bind _overheatbar_mat (`self.OverheatBar Mat`))
  (`/Engine/EditorBlueprintResources/StandardMacros.IsValid` _overheatbar_mat
    (:`Is Valid`
      (`MaterialInstanceDynamic.SetScalarParameterValue` _overheatbar_mat "Progress" Progress)
      (`MaterialInstanceDynamic.SetScalarParameterValue` _overheatbar_mat "Overheat" (`KismetMathLibrary.SelectFloat` 1.0 0.0 Overheated)))))

(fn `UserConstructionScript`)