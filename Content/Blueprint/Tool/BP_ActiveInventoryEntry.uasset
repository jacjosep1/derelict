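; BP_ActiveInventoryEntry tracks the heat state of the tool held in an active inventory entry.
; CoolHeat lowers heat over time by the tool's cooling rate without dropping below zero, while AddHeat raises it by a given amount.
; Reaching the overheat threshold sets heat to that threshold plus the tool's penalty, lengthening recovery.
; HeatInfo reports the current heat and whether the tool is overheated.
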(fn `Add Heat`
  (params (Amount :type "Float (double-precision)"))
  (bind _output_get (set `self.Current Heat` (+ (`self.Current Heat`) Amount)))
  (if (>= _output_get 1.0)
    (set `self.Current Heat` (+ 1.0 (`/Game/Blueprint/Tool/BP_Tool.Heat Penality` (`self.Tool`))))))

(fn `Cool Heat`
  (params (dt :type "Float (double-precision)"))
  (`/Engine/EditorBlueprintResources/StandardMacros.IsValid` (`self.Tool`)
    (:`Is Valid`
      (set `self.Current Heat` (`KismetMathLibrary.FClamp` (- (`self.Current Heat`) (* dt (`/Game/Blueprint/Tool/BP_Tool.CoolingRate` (`self.Tool`)))) 0.0 999.0)))))

(fn `Heat Info`
  (returns (Overheated :type Boolean) (`Current Heat` :type "Float (double-precision)"))
  (return (>= (`self.Current Heat`) 1.0) (`self.Current Heat`)))